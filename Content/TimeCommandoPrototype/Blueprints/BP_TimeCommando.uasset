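; BP_TimeCommando is a top-down player character that aims at the mouse cursor while moving relative to the camera.
; Movement input uses the Playerview camera's forward and right vectors flattened to the ground, and TurnRight rotates the spring arm in yaw.
; Each tick, a trace under the cursor drives the mesh's interpolated facing and eases the spring arm toward that point, clamped to a maximum offset.
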(event `InputAxis|TurnRight`
  (params (AxisValue :type "Float (single-precision)"))
  (`SceneComponent.K2_AddWorldRotation` (`self.SpringArm`) (`KismetMathLibrary.MakeRotator` 0.0 0.0 (* AxisValue (`self.CameraRotationSpeed`))) false false))

(event `InputAxis|MoveForward`
  (params (AxisValue :type "Float (single-precision)"))
  (bind (_returnvalue_x _returnvalue_y) (`KismetMathLibrary.BreakVector` (`SceneComponent.GetForwardVector` (`self.Playerview`))))
  (`self.AddMovementInput` (`KismetMathLibrary.Normal` (`KismetMathLibrary.MakeVector` _returnvalue_x _returnvalue_y)) AxisValue))

(event `InputAxis|MoveRight`
  (params (AxisValue :type "Float (single-precision)"))
  (bind (_returnvalue_x _returnvalue_y) (`KismetMathLibrary.BreakVector` (`SceneComponent.GetRightVector` (`self.Playerview`))))
  (`self.AddMovementInput` (`KismetMathLibrary.Normal` (`KismetMathLibrary.MakeVector` _returnvalue_x _returnvalue_y)) AxisValue))

(event `self.ReceiveTick`
  (params (DeltaSeconds :type "Float (single-precision)"))
  (`self.SetMeshRotation` DeltaSeconds)
  (`self.SetCameraOffset` DeltaSeconds))

(fn `SetCameraOffset`
  (params (DeltaTime :type "Float (double-precision)"))
  (`SceneComponent.K2_SetRelativeLocation` (`self.SpringArm`) (`KismetMathLibrary.ClampVectorSize` (`KismetMathLibrary.VInterpTo` (`SceneComponent.RelativeLocation` (`self.SpringArm`)) (* (- (`.Location` (`GameplayStatics.BreakHitResult` (`PlayerController.GetHitResultUnderCursorByChannel` (`GameplayStatics.GetPlayerController` 0) "TraceTypeQuery1" true))) (`self.K2_GetActorLocation`)) (`self.OffsetScale`)) DeltaTime (`self.OffsetSpeed`)) 0.0 (`self.MaxCameraOffset`)) false false))

(fn `SetMeshRotation`
  (params (`Delta Time` :type "Float (double-precision)"))
  (bind (_returnvalue_roll _returnvalue_pitch _returnvalue_yaw) (`KismetMathLibrary.BreakRotator` (`KismetMathLibrary.FindLookAtRotation` (`self.K2_GetActorLocation`) (`.Location` (`GameplayStatics.BreakHitResult` (`PlayerController.GetHitResultUnderCursorByChannel` (`GameplayStatics.GetPlayerController` 0) "TraceTypeQuery1" true))))))
  (`SceneComponent.K2_SetWorldRotation` (`self.Mesh`) (`KismetMathLibrary.RInterpTo` (`SceneComponent.K2_GetComponentRotation` (`self.Mesh`)) (`KismetMathLibrary.MakeRotator` 0.0 0.0 (+ _returnvalue_yaw -90.0)) `Delta Time` (`self.RotationSpeed`)) false false))

(fn `UserConstructionScript`)