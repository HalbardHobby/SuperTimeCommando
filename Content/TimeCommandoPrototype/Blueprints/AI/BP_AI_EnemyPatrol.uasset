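; AI controller for patrolling enemies that tracks the player through perception and blackboard keys.
; Perception updates write whether the stored Enemy was successfully sensed, using its first stimulus.
; Helper functions write the enemy, state and first patrol location from the controlled BP_Enemy to the blackboard.
; The setup chain that starts BT_EnemyPatrol and calls these helpers is disconnected, and BeginPlay is empty.
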(event `self.ReceiveBeginPlay`)

(event `self.AIPerception.OnPerceptionUpdated`
  (params (UpdatedActors :type "Array of Actor Object Reference (by ref)"))
  (for _array_element UpdatedActors
    (if (== _array_element (`self.Enemy`))
      (bind _info (`AIPerceptionComponent.GetActorsPerception` (`self.AIPerception`) _array_element))
      (bind (_output_age _output_expirationage _output_strength _output_stimuluslocation _output_receiverlocation _output_tag _output_bsuccessfullysensed) (break `AIStimulus` (`|GetArrayItem` (`.LastSensedStimuli` (break `ActorPerceptionBlueprintInfo` _info)))))
      (`BlackboardComponent.SetValueAsBool` (`AIBlueprintHelperLibrary.GetBlackboard` null) (`self.BlackboardKeyIsEnemyVisible`) _output_bsuccessfullysensed))))

(fn `SetEnemy`
  (params (`New Enemy` :type "Pawn Object Reference"))
  (locals (BlackboardKeyEnemy :type Name :default "Enemy") (BlackboardKeyState :type Name :default "CurrentState") (NewLocalVar_0 :type Byte :default 1))
  (bind _returnvalue (`AIBlueprintHelperLibrary.GetBlackboard` null))
  (if (!= `New Enemy` (`self.Enemy`))
    (bind _asbp_time_commando_player (cast `/Game/SuperTimeCommando/Chaacters/BP_TimeCommandoPlayer` `New Enemy`))
    (bind _output_get (set `self.Enemy` _asbp_time_commando_player))
    (`BlackboardComponent.SetValueAsObject` _returnvalue (`local.BlackboardKeyEnemy`) _output_get)
    (`BlackboardComponent.SetValueAsEnum` _returnvalue (`local.BlackboardKeyState`) (`local.NewLocalVar_0`))))

(fn `SetFirstPatrolPoint`
  (locals (PawnBlackboardKey :type Name :default "None"))
  (bind _asbp_enemy (cast `/Game/SuperTimeCommando/Chaacters/BP_Enemy` (`self.K2_GetPawn`)))
  (bind _returnvalue (`EnemyPatrol.GetNextPatrolPoint` _asbp_enemy))
  (`BlackboardComponent.SetValueAsVector` (`AIBlueprintHelperLibrary.GetBlackboard` null) (`self.NextLocationBlackboardKey`) (`self.K2_GetActorLocation` _returnvalue)))

(fn `UserConstructionScript`)