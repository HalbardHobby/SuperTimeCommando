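; Component that records its owner's transform over time and moves the owner back along that path during a time rewind.
; Tick samples transforms after a delay, drawing debug frustums; past the TotalRewind-based cap it removes the newest entry instead of adding.
; Start/stop events bound on TimeCommandoControllerBP toggle recording and rewinding.
; Rewinding lerps toward each saved transform from the last backward, removing it when nearly reached and stopping at index zero.
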(event `self.ReceiveTick`
  (params (DeltaSeconds :type "Float (single-precision)"))
  (bind _returnvalue (`self.GetOwner`))
  (bind _locationframes (`self.LocationFrames`))
  (bind _counter (`self.Counter`))
  (bind _locationframes_2 (`self.LocationFrames`))
  (bind _returnvalue_2 (`Actor.GetTransform` _returnvalue))
  (bind _output (`|GetArrayItem` (`self.LocationFrames`) (`self.Counter`)))
  (set `self.DeltaTime` DeltaSeconds)
  (`|ExecutionSequence`
    (:`then_0`
      (if (`self.CanSetFrame`)
        (`KismetSystemLibrary.Delay` (`self.TimeBetweenFrames`))
        (if (> (`KismetArrayLibrary.Array_Length` _locationframes) (`KismetMathLibrary.FTrunc` (/ (`self.TotalRewind`) (`self.TimeBetweenFrames`))))
          (`KismetArrayLibrary.Array_Remove` _locationframes (`KismetArrayLibrary.Array_LastIndex` _locationframes))
          (else
            (bind _returnvalue_3 (`KismetArrayLibrary.Array_Add` _locationframes_2 (`Actor.GetTransform` (`self.GetOwner`))))
            (`KismetSystemLibrary.DrawDebugFrustum` (`|GetArrayItem` _locationframes_2 _returnvalue_3) (struct :`R` 1.0 :`B` 0.126024 :`A` 1.0) 6.0 15.0)))))
    (:`then_1`
      (if (`self.IsRewinding`)
        (`Actor.K2_SetActorTransform` _returnvalue (`KismetMathLibrary.TLerp` _returnvalue_2 _output (* (`self.DeltaTime`) (`self.TravelSpeed`))) false false)
        (if (`KismetMathLibrary.NearlyEqual_TransformTransform` _returnvalue_2 _output 100.0 100.0 100.0)
          (`KismetArrayLibrary.Array_Remove` (`self.LocationFrames`) _counter)
          (`/Engine/EditorBlueprintResources/StandardMacros.DecrementInt` _counter
            (:`  `
              (if (== _counter 0)
                (set `self.IsRewinding` false)))))))))

(event `self.ReceiveBeginPlay`
  (bind _astime_commando_controller_bp (cast `/Game/TimeCommandoPrototype/Blueprints/TimeCommandoControllerBP` (`GameplayStatics.GetPlayerController` 0)))
  (add `/Game/TimeCommandoPrototype/Blueprints/TimeCommandoControllerBP.StartRewind` _astime_commando_controller_bp (delegate `StartRewind`))
  (add `/Game/TimeCommandoPrototype/Blueprints/TimeCommandoControllerBP.StopRewind` _astime_commando_controller_bp (delegate `StopRewind`)))

(event `StopRewind`
  (set `self.CanSetFrame` true)
  (set `self.IsRewinding` false))

(event `StartRewind`
  (set `self.Counter` (`KismetArrayLibrary.Array_LastIndex` (`self.LocationFrames`)))
  (set `self.CanSetFrame` false)
  (set `self.IsRewinding` true))